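; BP_Paper_memo_3 is an obtainable memo object, the third one, that gives the player a rough view of the game's world.
; BeginPlay creates the BPI_paperStory3 widget and stores it.
; Releasing E while IsView is true calls ShowUI3, which adds the widget to the viewport, shows the cursor and switches to UI-only input.
; Nothing in these graphs initially sets IsView true outside ShowUI3 itself.
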(event `self.ReceiveBeginPlay`
  (`parent.ReceiveBeginPlay`)
  (bind _returnvalue (`|CreateWidget` "/Game/Developers/haeun/Collections/Blueprint/Hint/BPI_paperStory3.BPI_paperStory3_C"))
  (set `self.paperMemo3` _returnvalue))

(event `Key|E`
  (params (Key :type "Key Structure"))
  ;[1 1 1] 대략적인 세계관을 알 수 있는 메모3, 획득 오브젝트
  (:`Released`
    (if (`self.IsView`)
      (`self.ShowUI3` (`self.paperMemo3`))
      (else
        (set `self.IsView` false)))))

(fn `ShowUI3`
  (params (target :type "UserWidget Object Reference"))
  (bind _returnvalue (`GameplayStatics.GetPlayerController` 0))
  (set `PlayerController.bShowMouseCursor` true _returnvalue)
  (`WidgetBlueprintLibrary.SetInputMode_UIOnlyEx` _returnvalue null)
  (`UserWidget.AddToViewport` target 0)
  (set `self.IsView` true)
  (return))

(fn `UserConstructionScript`
  (`parent.UserConstructionScript`))
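; BP_Paper_memo_2 is an obtainable paper memo, the second one, that reveals rough background on the game's world.
; BeginPlay creates the BPI_paperStory2 widget once and stores it as PaperMemo.
; EClick calls ShowUIMemo2 only when IsView is already true, otherwise setting it false.
; ShowUIMemo2 shows the cursor, switches to UI-only input, adds the widget to the viewport and sets IsView true.
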(event `self.ReceiveBeginPlay`
  (`parent.ReceiveBeginPlay`)
  (bind _returnvalue (`|CreateWidget` "/Game/Blueprints/BPI_paperStory2.BPI_paperStory2_C"))
  (set `self.PaperMemo` _returnvalue))

(event `/Game/Developers/haeun/Collections/Blueprint/EClickBPI.EClick`
  ;[1 1 1] 대략적인 세계관을 알 수 있는 메모2, 획득 오브젝트
  (if (`self.IsView`)
    (`self.ShowUIMemo2` (`self.PaperMemo`))
    (else
      (set `self.IsView` false))))

(fn `ShowUIMemo2`
  (params (target :type "UserWidget Object Reference"))
  (bind _returnvalue (`GameplayStatics.GetPlayerController` 0))
  (set `PlayerController.bShowMouseCursor` true _returnvalue)
  (`WidgetBlueprintLibrary.SetInputMode_UIOnlyEx` _returnvalue null)
  (`UserWidget.AddToViewport` target 0)
  (set `self.IsView` true)
  (return))

(fn `UserConstructionScript`
  (`parent.UserConstructionScript`))
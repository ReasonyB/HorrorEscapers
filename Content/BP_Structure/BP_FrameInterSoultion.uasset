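; BP_FrameInterSoultion is an interactable picture frame slot for a puzzle in the Escapers game.
; On left-click it runs the parent interaction, plays a sound and clears Install if that flag is set, then reports its Index and Right value to GM_Escapers through SetPictures.
; It binds to the game mode's PicturesIsClear event, which sets UsedOnce and blocks further clicks once the pictures are solved.
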(event `self.ReceiveBeginPlay`
  (`parent.ReceiveBeginPlay`)
  (bind _asgm_escapers (cast `/Game/Blueprints/PlayerSystem/GM_Escapers` (`GameplayStatics.GetGameMode`)))
  (add `/Game/Blueprints/PlayerSystem/GM_Escapers.Pictures is Clear` _asgm_escapers (delegate `Pictures are clear`)))

(event `Pictures are clear`
  (set `self.Used Once` true))

(event `/Game/Blueprints/BPI_MouseInputs.좌클릭일 때`
  (if (not (`self.Used Once`))
    (`parent.좌클릭일 때`)
    (if (`self.Install?`)
      (`AudioComponent.Play` (`self.Sound Effect`) 0.0)
      (set `self.Install?` false))
    (bind _asgm_escapers (cast `/Game/Blueprints/PlayerSystem/GM_Escapers` (`GameplayStatics.GetGameMode`)))
    (`/Game/Blueprints/PlayerSystem/GM_Escapers.Set Pictures` _asgm_escapers (`self.Index`) (`self.right?`))))

(fn `UserConstructionScript`
  (`parent.UserConstructionScript`))
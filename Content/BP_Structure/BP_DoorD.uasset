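; BP_DoorD is a door actor that swings open when its DoorisOpen event is called.
; It caches the current yaw, then a RotateZ timeline offsets it by up to -90 degrees through relative rotation.
; The timeline's Sound event track plays the sound effect and passes the OpenDoor2 speech from DT_Monologue to BP_PlayerState to start a monologue.
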(event `Door is Open`
  (bind (_returnvalue_roll _returnvalue_pitch _returnvalue_yaw) (`KismetMathLibrary.BreakRotator` (`self.K2_GetActorRotation`)))
  (set `self.World Rotate` _returnvalue_yaw)
  (bind (_direction _z) (`Timeline|RotateZ`)
    (:`Update`
      (`self.K2_SetActorRelativeRotation` (`KismetMathLibrary.MakeRotator` 0.0 0.0 (+ (`self.World Rotate`) (* -90 _z)))))
    (:`Sound`
      (`AudioComponent.Play` (`self.Sound effect`) 0.0)
      (bind _asbp_player_state (cast `/Game/Blueprints/PlayerSystem/BP_PlayerState` (`Pawn.PlayerState` (`GameplayStatics.GetPlayerCharacter` 0))))
      (bind _returnvalue (`|GetDataTableRow` "/Game/Blueprints/DT_Monologue.DT_Monologue" "OpenDoor2")
        (:`then`
          (set `/Game/Blueprints/PlayerSystem/BP_PlayerState.Monologue` (`|MakeArray` (break `/Game/Blueprints/ST_Monologue` _returnvalue)) _asbp_player_state)
          (`/Game/Blueprints/PlayerSystem/BP_PlayerState.Set First Monologue` _asbp_player_state))))))

(fn `UserConstructionScript`)
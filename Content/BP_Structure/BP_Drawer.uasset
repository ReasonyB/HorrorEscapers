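; BP_Drawer is a drawer that slides open and closed on a left-click event, locked until a number-key puzzle is solved.
; The click handler checks NumberKeySuccess on the GM_Escapers game mode before doing anything.
; A FlipFlop alternates playing and reversing the Move timeline, which lerps InteractionPoint's relative location between two stored drawer vectors without sweep.
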(event `/Game/Blueprints/BPI_MouseInputs.좌클릭일 때`
  (bind _asgm_escapers (cast `/Game/Blueprints/PlayerSystem/GM_Escapers` (`GameplayStatics.GetGameMode`)))
  (if (`/Game/Blueprints/PlayerSystem/GM_Escapers.NumberKeySuccess` _asgm_escapers)
    (`/Engine/EditorBlueprintResources/StandardMacros.FlipFlop`
      (:`A`
        (bind (_direction _move) (`Timeline|Move` :!label _label)
          (:`Update`
            (`SceneComponent.K2_SetRelativeLocation` (`self.Interaction Point`) (`KismetMathLibrary.VLerp` (`self.DrawerCurrentVector`) (`self.DrawerNewtVector`) _move) false false))))
      (:`B`
        (goto _label :!via `Reverse`)))))

(fn `UserConstructionScript`)
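; BP_Lock is a padlock actor that opens with the correct answer to Quiz 1.
; On BeginPlay it creates a BPI_LockUI1 widget and passes it CorrectAnswer.
; The left-click event shows the widget with mouse cursor and UI-only input, while a repeat click only clears the IsView flag.
; Tick polls NumberKeySuccess on the GM_Escapers game mode and destroys the lock once it is true.
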(event `self.ReceiveTick`
  (params (DeltaSeconds :type "Float (single-precision)"))
  (`parent.ReceiveTick` DeltaSeconds)
  (bind _asgm_escapers (cast `/Game/Blueprints/PlayerSystem/GM_Escapers` (`GameplayStatics.GetGameMode`)))
  (if (`/Game/Blueprints/PlayerSystem/GM_Escapers.NumberKeySuccess` _asgm_escapers)
    (`self.K2_DestroyActor`)))

(event `self.ReceiveBeginPlay`
  ;[1 1 1] 퀴즈1 정답을 통해 열수있는 자물쇠
  (`parent.ReceiveBeginPlay`)
  (bind _returnvalue (`|CreateWidget` "/Game/Blueprints/UI/BPI_LockUI1.BPI_LockUI1_C"))
  (bind _output_get (set `self.BPI_LockUI` _returnvalue))
  (set `/Game/Blueprints/UI/BPI_LockUI1.Answer` (`self.CorrectAnswer`) _output_get))

(event `/Game/Blueprints/BPI_MouseInputs.좌클릭일 때`
  (bind _returnvalue (`GameplayStatics.GetPlayerController` 0))
  (if (`self.IsView`)
    (set `self.IsView` false)
    (else
      (set `PlayerController.bShowMouseCursor` true _returnvalue)
      (`WidgetBlueprintLibrary.SetInputMode_UIOnlyEx` _returnvalue null)
      (`UserWidget.AddToViewport` (`self.BPI_LockUI`) 0)
      (set `self.IsView` true))))

(fn `UserConstructionScript`
  (`parent.UserConstructionScript`))
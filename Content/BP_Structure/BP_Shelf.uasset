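; BP_Shelf is a shelf actor that slides along its local X axis when its DoorisOpen event fires.
; The event plays a timeline whose VecAddX track feeds AddActorLocalTransform on each update, so the movement accumulates as incremental offsets rather than interpolating between fixed positions.
; A Sound Track event on the same timeline starts the MPSpinning sound.
; BeginPlay, overlap and Tick are disabled stubs.
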(event `Door is Open`
  (bind (_direction _vecaddx) (`Timeline|타임라인_0`)
    (:`Update`
      (`self.K2_AddActorLocalTransform` (`KismetMathLibrary.MakeTransform` (`KismetMathLibrary.MakeVector` _vecaddx) (struct) (0.8 0.8 0.8))))
    (:`Sound Track`
      (`AudioComponent.Play` (`self.MP_Spinning_`) 0.0))))

(fn `UserConstructionScript`
  (`parent.UserConstructionScript`))
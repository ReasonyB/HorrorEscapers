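; BP_PipeUITrigger is a trigger that opens a pipe UI widget, apparently a puzzle, on left click.
; BeginPlay creates the BPI_pipeUI1 widget once and passes it the trigger's PipeAnswer.
; The click event (좌클릭일때) toggles IsView: when false, it adds the widget to the viewport with UI-only input and a visible cursor.
; When true, it only clears the flag, without removing the widget or restoring input.
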(event `self.ReceiveBeginPlay`
  (bind _returnvalue (`|CreateWidget` "/Game/Developers/haeun/Collections/Blueprint/Pipe/BPI_pipeUI1.BPI_pipeUI1_C"))
  (bind _output_get (set `self.PipeUI` _returnvalue))
  (set `/Game/Developers/haeun/Collections/Blueprint/Pipe/BPI_pipeUI1.Answer` (`self.PipeAnswer`) _output_get))

(event `/Game/Blueprints/BPI_MouseInputs.좌클릭일 때`
  (bind _returnvalue (`GameplayStatics.GetPlayerController` 0))
  (if (`self.IsView`)
    (set `self.IsView` false)
    (else
      (set `PlayerController.bShowMouseCursor` false _returnvalue)
      (`WidgetBlueprintLibrary.SetInputMode_UIOnlyEx` _returnvalue (`self.PipeUI`))
      (set `PlayerController.bShowMouseCursor` true (`GameplayStatics.GetPlayerController` 0))
      (`UserWidget.AddToViewport` (`self.PipeUI`) 0)
      (set `self.IsView` true))))

(fn `UserConstructionScript`)
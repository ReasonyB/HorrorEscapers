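; BP_Item is a parent Blueprint for pickup items that add themselves to the player's inventory through BP_PlayerState.
; On BeginPlay it stores its own class in the Info struct alongside the item id, which SetInfoById can change.
; The left-click event passes Info to AddItem, then plays a pickup sound and destroys the actor when that call returns false.
; SetPhysics enables physics simulation on the Trigger component.
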(event `self.ReceiveBeginPlay`
  (bind _info_id (break `/Game/Blueprints/ParentClasses/etc/ST_Item` (`self.Info`)))
  (set `self.Info` (make `/Game/Blueprints/ParentClasses/etc/ST_Item` _info_id (`GameplayStatics.GetObjectClass` self))))

(event `/Game/Blueprints/BPI_MouseInputs.좌클릭일 때`
  (bind _asbp_player_state (cast `/Game/Blueprints/PlayerSystem/BP_PlayerState` (`Pawn.PlayerState` (`GameplayStatics.GetPlayerCharacter` 0))))
  (bind _can_t_add (`/Game/Blueprints/PlayerSystem/BP_PlayerState.AddItem` _asbp_player_state (`self.Info`)))
  (if (not _can_t_add)
    (`GameplayStatics.PlaySound2D` "/Engine/VREditor/Sounds/UI/Object_PickUp.Object_PickUp" 1.0 1.0 0.0 null null)
    (`self.K2_DestroyActor`)))

(fn `Set Info by id`
  (params (`Info Id` :type Integer))
  (bind (_info_id _info_classtype) (break `/Game/Blueprints/ParentClasses/etc/ST_Item` (`self.Info`)))
  (set `self.Info` (make `/Game/Blueprints/ParentClasses/etc/ST_Item` `Info Id` _info_classtype)))

(fn `Set Physics`
  (`PrimitiveComponent.SetSimulatePhysics` (`self.Trigger`) true))

(fn `UserConstructionScript`)
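; Blueprint function library that supplies the monologue lines for hint paper and memo finds.
; Each item has its own function that looks up hard-coded rows in DT_Monologue and returns their Speech values as an array of one or two lines.
; Memo3 reads the ThirdMemoFind1 row twice, so both of its entries are identical.
; No function handles a missing row.
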(fn `HintPaper1`
  (returns (Array :type "Array of String"))
  (bind _returnvalue (`|GetDataTableRow` "/Game/Blueprints/DT_Monologue.DT_Monologue" "FirstHintFind1")
    (:`then`
      (return (`|MakeArray` (break `/Game/Blueprints/ST_Monologue` _returnvalue))))))

(fn `HintPaper2`
  (returns (Array :type "Array of String"))
  (bind _returnvalue (`|GetDataTableRow` "/Game/Blueprints/DT_Monologue.DT_Monologue" "SecondHintFind1")
    (:`then`
      (bind _returnvalue_2 (`|GetDataTableRow` "/Game/Blueprints/DT_Monologue.DT_Monologue" "SecondHintFind2")
        (:`then`
          (return (`|MakeArray` (break `/Game/Blueprints/ST_Monologue` _returnvalue) (break `/Game/Blueprints/ST_Monologue` _returnvalue_2))))))))

(fn `Memo1`
  (returns (Array :type "Array of String"))
  (bind _returnvalue (`|GetDataTableRow` "/Game/Blueprints/DT_Monologue.DT_Monologue" "FirstMemoFind1")
    (:`then`
      (return (`|MakeArray` (break `/Game/Blueprints/ST_Monologue` _returnvalue))))))

(fn `Memo2`
  (returns (Array :type "Array of String"))
  (bind _returnvalue (`|GetDataTableRow` "/Game/Blueprints/DT_Monologue.DT_Monologue" "SecondMemoFind1")
    (:`then`
      (bind _returnvalue_2 (`|GetDataTableRow` "/Game/Blueprints/DT_Monologue.DT_Monologue" "SecondMemoFind2")
        (:`then`
          (return (`|MakeArray` (break `/Game/Blueprints/ST_Monologue` _returnvalue) (break `/Game/Blueprints/ST_Monologue` _returnvalue_2))))))))

(fn `Memo3`
  (returns (Array :type "Array of String"))
  (bind _returnvalue (`|GetDataTableRow` "/Game/Blueprints/DT_Monologue.DT_Monologue" "ThirdMemoFind1")
    (:`then`
      (bind _returnvalue_2 (`|GetDataTableRow` "/Game/Blueprints/DT_Monologue.DT_Monologue" "ThirdMemoFind1")
        (:`then`
          (return (`|MakeArray` (break `/Game/Blueprints/ST_Monologue` _returnvalue) (break `/Game/Blueprints/ST_Monologue` _returnvalue_2))))))))
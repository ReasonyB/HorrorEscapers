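; Player state Blueprint that manages the player's hotbar inventory: selecting, adding, using and dropping items.
; Hotbar holds item structs alongside a parallel ItemCount array, stacking known items and placing new ones in empty slots (Id -1).
; A full hotbar shows a timed monologue line from DT_Monologue, while dispatchers announce slot changes.
; TakeOutItem spawns the current item as a physics actor, then UseItem decrements its count and clears depleted slots.
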(event `self.ReceiveBeginPlay`
  (`KismetArrayLibrary.Array_Resize` (`self.ItemCount`) (`KismetArrayLibrary.Array_Length` (`self.Hotbar`))))

(fn `AddItem`
  (params (item :type "/Game/Blueprints/ParentClasses/etc/ST_Item Structure"))
  (returns (`Can't Add` :type Boolean))
  (locals (`Slot Index` :type Integer :default -1) (Count :type Integer))
  (bind (_is_contain _index) (`self.Check In Belongings` item))
  (bind _returnvalue (`KismetArrayLibrary.Array_Find` (`self.Hotbar`) (make `/Game/Blueprints/ParentClasses/etc/ST_Item` -1)))
  (if _is_contain
    (bind _output_get (set `local.Slot Index` _index))
    (`KismetArrayLibrary.Array_Set` (`self.ItemCount`) _output_get (+ (`|GetArrayItem` (`self.ItemCount`) (`local.Slot Index`)) 1))
    (elif (`KismetArrayLibrary.Array_IsValidIndex` (`self.Hotbar`) _returnvalue)
      (bind _output_get_2 (set `local.Slot Index` _returnvalue))
      (`KismetSystemLibrary.PrintText` (`|FormatText` "Index to Add: {0}" _output_get_2) true true (struct :`R` 1.0 :`B` 0.123857 :`A` 1.0) 10.0)
      (`KismetArrayLibrary.Array_Set` (`self.Hotbar`) _output_get_2 item)
      (bind _output_get_3 (set `local.Count` 1))
      (`KismetArrayLibrary.Array_Set` (`self.ItemCount`) _output_get_2 _output_get_3)
      (`self.Add Item To HotBar` (`local.Slot Index`) item)
      (else
        (bind _returnvalue_2 (`|GetDataTableRow` "/Game/Blueprints/DT_Monologue.DT_Monologue" "FullInventory")
          (:`then`
            (set `self.Monologue` (break `/Game/Blueprints/ST_Monologue` _returnvalue_2))
            (`KismetSystemLibrary.K2_SetTimer` null "Reset Monologue" 1.0)
            (return true))))))
  (`self.Debug Inventory`)
  (return false))

(fn `ChooseItem`
  (params (index :type Integer))
  (if (and (`KismetArrayLibrary.Array_IsValidIndex` (`self.Inventory`) index) (!= (`self.currentItem`) index))
    (`self.Choose HotBar` (`self.currentItem`) index)
    (bind _output_get (set `self.currentItem` index))
    (`KismetSystemLibrary.PrintString` (`KismetStringLibrary.Conv_IntToString` _output_get))))

(fn `Debug Inventory`
  (for (_array_element _array_index) (`self.Hotbar`)
    (`KismetSystemLibrary.PrintText` (`|FormatText` "Item[{0}], {class} 클래스, {id} : {1} 개 보유중" _array_index (`KismetSystemLibrary.GetClassDisplayName` (`.classType_5_1BED948A43758C64FC8922B4EEBFBCE2` (break `/Game/Blueprints/ParentClasses/etc/ST_Item` _array_element))) (break `/Game/Blueprints/ParentClasses/etc/ST_Item` _array_element) (`BlueprintMapLibrary.Map_Find` (`self.itemQuantity`) (break `/Game/Blueprints/ParentClasses/etc/ST_Item` _array_element))) true true (struct :`G` 0.66 :`B` 1.0 :`A` 1.0) 10.0)))

(fn `Get Current Item`
  (returns (Output :type "/Game/Blueprints/ParentClasses/etc/ST_Item Structure"))
  (return (`self.Get Current Item Info`)))

(fn `Reset Monologue`
  (set `self.Monologue` ""))

(fn `Take Out Item`
  (params (SpawnTransform :type "Transform Structure"))
  (locals (curid :type Integer))
  (bind (_output_id _output_classtype) (break `/Game/Blueprints/ParentClasses/etc/ST_Item` (`self.Get Current Item Info`)))
  (if (!= _output_classtype null)
    (set `local.curid` _output_id)
    (bind _returnvalue (`|SpawnActorFromClass` _output_classtype SpawnTransform "AdjustIfPossibleButAlwaysSpawn" "OverrideRootScale" null null))
    (`/Game/Blueprints/ParentClasses/BP_Item.Set Info by id` _returnvalue (`local.curid`))
    (`/Game/Blueprints/ParentClasses/BP_Item.Set Physics` _returnvalue)
    (`self.Use Item`)
    (`GameplayStatics.PlaySound2D` "/Game/HorrorEngine/Audio/Environment/PickUp.PickUp" 1.0 1.0 0.0 null null)))

(fn `Use Item`
  (bind _returnvalue (- (`self.Get Current Item Count`) 1))
  (`KismetArrayLibrary.Array_Set` (`self.ItemCount`) (`self.currentItem`) _returnvalue)
  (if (<= _returnvalue 0)
    ;[1 1 1] 아이템 창에서 삭제 및 수집 가능 상태로 초기화
    (`KismetArrayLibrary.Array_Set` (`self.Hotbar`) (`self.currentItem`) (make `/Game/Blueprints/ParentClasses/etc/ST_Item` -1))
    (`self.Take Out Item From HotBar` (`self.currentItem`))))

(fn `UserConstructionScript`)
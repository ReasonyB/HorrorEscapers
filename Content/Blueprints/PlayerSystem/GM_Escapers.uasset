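; GM_Escapers, apparently the game mode for an escape game, runs a countdown and tracks a pipe puzzle.
; BeginPlay builds a Timespan timer from TimeLimit, and Tick accumulates delta time to subtract whole seconds; the expiry branch is empty.
; SetPipe writes into the CheckPipes boolean array at valid indices, then CheckAnswers ANDs all entries to detect a solved puzzle, which is only reported by a debug print.
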(event `self.ReceiveBeginPlay`
  (set `self.Timer` (`KismetMathLibrary.MakeTimespan` 0 0 (`self.TimeLimit`))))

(event `self.ReceiveTick`
  (params (DeltaSeconds :type "Float (single-precision)"))
  (bind _output_get (set `self.Delta Seconds` (+ DeltaSeconds (`self.Delta Seconds`))))
  (if (>= _output_get 1.0)
    (set `self.Timer` (- (`self.Timer`) (`KismetMathLibrary.MakeTimespan` 0 0 0 1)))
    (set `self.Delta Seconds` (- (`self.Delta Seconds`) 1.0))
    (if (< (`self.Timer`) (struct))
      _)))

(fn `Check Answers`
  (params (`Setting Arrays` :type "Array of Boolean"))
  (locals (`is Correct` :type Boolean :default true))
  (for _array_element `Setting Arrays`
    (set `local.is Correct` (and _array_element (`local.is Correct`))))
  (if (`local.is Correct`)
    (return)))

(fn `Set Pipe`
  (params (Index :type Integer) (Item :type "Boolean (by ref)"))
  (bind _check_pipes (`self.Check Pipes`))
  (if (`KismetArrayLibrary.Array_IsValidIndex` _check_pipes Index)
    (`KismetArrayLibrary.Array_Set` _check_pipes Index Item)
    (`self.Check Answers` (`self.Check Pipes`))
    (`KismetSystemLibrary.PrintString` "Pipes is Correct")))

(fn `UserConstructionScript`)